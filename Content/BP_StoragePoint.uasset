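; BP_StoragePoint is a storage point that counts ore dropped at it and shows the total on a text render.
; The count resets to zero at BeginPlay.
; The DoAction event switches on its Operation argument, and the Drop case increments NumOre and writes the formatted count to TextRender1.
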(event EventBeginPlay
  (|CallParentFunction)
  (Variables|Default|SetNumOre 0))

(event EventDoAction
  (params (Operation :type EMinerTaskOperator%20Enum :default "Drop"))
  (switch Utilities|FlowControl|Switch|SwitchonEMinerTaskOperator Operation
    (:Drop
      (bind _result (Math|Integer|IncrementInt (Variables|Default|GetNumOre))
        (:%20%20
          (Rendering|Components|TextRender|SetText (Variables|Default|GetTextRender1) (Utilities|Text|FormatText "Ore : {0}" _result)))))))

(fn ConstructionScript
  (|CallParentFunction))