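; BP_Agent is a miner AI agent that plans its tasks with a Hierarchical Task Network and carries them out.
; On BeginPlay it seeds the ore and tool world state in BasicHTNBrain and stores the planned action sequence.
; Actions run sequentially: navigation uses AIMoveTo toward storage, tool storage or mine points, while pickup and drop call the destination BP_ActionPoint, then wait briefly.
; Each completed action advances the index until Finish resets it, without replanning.
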(event Custom|NavigateActionEvent
  (params (ActionParam :type EMinerTaskOperatorParam%20Enum :default "Ore"))
  ;[1 1 1] Actions
  ;;[1 1 1] NavigateTo Action
  (Development|PrintString (Utilities|String|Append "Navigate " (Utilities|String|EnumtoString ActionParam)))
  (switch Utilities|FlowControl|Switch|SwitchonEMinerTaskOperatorParam ActionParam
    (:Storage
      (Variables|Default|SetDestinationActor (Variables|Default|GetStoragePoint)))
    (:ToolStorage
      (Variables|Default|SetDestinationActor (Variables|Default|GetToolStoragePoint)))
    (:Mine
      (Variables|Default|SetDestinationActor (Variables|Default|GetMinePoint))))
  (AI|AIMoveTo (AI|GetAIController self) "0, 0, 0" (Variables|Default|GetDestinationActor) -1.0 "Default" "Default" true true
    (:OnMoveFinished
      (CallFunction|FinishAction))))

(event Custom|DropActionEvent
  (params (ActionParam :type EMinerTaskOperatorParam%20Enum :default "Ore"))
  ;[1 1 1] Actions
  ;;[1 1 1] Drop Action
  (Development|PrintString (Utilities|String|Append "Drop " (Utilities|String|EnumtoString ActionParam)))
  (Default|DoAction (.AsBP%20Action%20Point (Utilities|Casting|CastToBP_ActionPoint (Variables|Default|GetDestinationActor))) "Drop")
  (Utilities|FlowControl|Delay 1.0)
  (CallFunction|FinishAction))

(event Custom|PickupActionEvent
  (params (ActionParam :type EMinerTaskOperatorParam%20Enum :default "Ore"))
  ;[1 1 1] Actions
  ;;[1 1 1] Pickup Action
  (Development|PrintString (Utilities|String|Append "Pickup " (Utilities|String|EnumtoString ActionParam)))
  (Default|DoAction (.AsBP%20Action%20Point (Utilities|Casting|CastToBP_ActionPoint (Variables|Default|GetDestinationActor))) "PickUp")
  (Utilities|FlowControl|Delay 1.0)
  (CallFunction|FinishAction))

(event Custom|FinishAction
  ;[1 1 1] Finish Action
  (if (< (Variables|Default|GetCurrentActionIndex) (Utilities|Array|Length (Variables|Default|GetActionSequence)))
    (Math|Integer|IncrementInt (Variables|Default|GetCurrentActionIndex)
      (:%20%20
        (CallFunction|DoActions)))))

(event Custom|DoActions
  ;[1 1 1] Do action sequence
  (switch Utilities|FlowControl|Switch|SwitchonEMinerTaskOperator (Utilities|Enum|ByteToEnumEMinerTaskOperator (.actionid (Utilities|Array|Get(acopy) (Variables|Default|GetActionSequence) (Variables|Default|GetCurrentActionIndex))))
    (:Drop
      (CallFunction|DropActionEvent (Utilities|Enum|ByteToEnumEMinerTaskOperatorParam (.actionparam (Utilities|Array|Get(acopy) (Variables|Default|GetActionSequence) (Variables|Default|GetCurrentActionIndex))))))
    (:PickUp
      (CallFunction|PickupActionEvent (Utilities|Enum|ByteToEnumEMinerTaskOperatorParam (.actionparam (Utilities|Array|Get(acopy) (Variables|Default|GetActionSequence) (Variables|Default|GetCurrentActionIndex))))))
    (:NavigateTo
      (CallFunction|NavigateActionEvent (Utilities|Enum|ByteToEnumEMinerTaskOperatorParam (.actionparam (Utilities|Array|Get(acopy) (Variables|Default|GetActionSequence) (Variables|Default|GetCurrentActionIndex))))))
    (:Finish
      (Variables|Default|SetCurrentActionIndex 0))))

(event EventBeginPlay
  (bind _basichtnbrain (Variables|Default|GetBasicHTNBrain))
  ;[1 1 1] Initialize & Planning
  (Class|BasicHTNBrainComponent|PopulateMinerWorldState _basichtnbrain (Utilities|Array|MakeArray (Utilities|Struct|MakeHTNWorldStateElem (Utilities|Enum|LiteralenumEMinerWorldState "HasOre") 0) (Utilities|Struct|MakeHTNWorldStateElem (Utilities|Enum|LiteralenumEMinerWorldState "HasTool") 0))) ; Initialize World State
  (bind _resultactionsequence (Class|BasicHTNBrainComponent|MinerHTNPlanning _basichtnbrain)) ; Do planning
  (Variables|Default|SetActionSequence _resultactionsequence)
  (Variables|Default|SetCurrentActionIndex 0)
  (CallFunction|DoActions))

(fn ConstructionScript)